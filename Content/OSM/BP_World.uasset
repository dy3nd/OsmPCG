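; World actor that builds a map area from OpenStreetMap road data around a hard-coded longitude/latitude.
; On BeginPlay it computes a bounding box and queries the Overpass API for highway ways through VaRest.
; The JSON response's geometry is converted via the GeoReferencing system into center-relative debug points, randomly coloured per way.
; It then moves itself to the box's minimum corner, generates a grid terrain mesh sized to the box and draws debug bounds.
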(event Custom|RequestComplete
  (params (Request :type Va%20Rest%20Request%20JSON%20Object%20Reference))
  (bind _bboxvectors (Variables|BBoxData|GetBBoxVectors))
  (bind _bboxvectors_2 (Variables|BBoxData|GetBBoxVectors))
  (bind _bboxvectors_3 (Variables|BBoxData|GetBBoxVectors))
  (bind _returnvalue (- (.x (.max (.vertices _bboxvectors_2))) (.x (.min (.vertices _bboxvectors_2)))))
  (bind _returnvalue_2 (- (.y (.max (.vertices _bboxvectors_2))) (.y (.min (.vertices _bboxvectors_2)))))
  ;[1 1 1] Get Response JSON
  (bind _returnvalue_3 (Class|VaRestRequestJSON|GetResponseContentasString Request false))
  (bind _outjsonobject (Class|JsonBlueprintFunctionLibrary|FromString _returnvalue_3))
  ;[1 1 1] Loop Through Elements
  (bind _outvalue (|GetJsonField _outjsonobject "elements"))
  (bind (_array_element _array_index) (Utilities|Array|ForEachLoopwithBreak _outvalue)
    (:LoopBody
      (CallFunction|HandlePOIGeometry (Math|Vector|MakeVector (.x (.center _bboxvectors_3)) (.y (.center _bboxvectors_3)) 0.0) (.geometry (Utilities|Struct|BreakS_POI _array_element))))
    (:Completed
      ;[1 1 1] Calc BBox Size KM²
      (Development|PrintString (Utilities|String|Append (Utilities|String|ToString(Float) _returnvalue) " by " (Utilities|String|ToString(Float) _returnvalue_2)) true true "(R=1.000000,G=0.868751,B=0.000000,A=1.000000)" 2e+02)
      (Variables|BBoxData|SetBBoxXLenghtCM _returnvalue)
      (Variables|BBoxData|SetBBoxYLenghtCM _returnvalue_2)
      (Development|PrintString "GenWorld")
      (Transformation|SetActorLocation (Math|Vector|MakeVector (- (.x (.min (.vertices _bboxvectors))) (.x (.center _bboxvectors))) (- (.y (.min (.vertices _bboxvectors))) (.y (.center _bboxvectors))) 0.0) false false)
      (Development|PrintString (Utilities|String|Append (Utilities|String|ToString(Integer) (Math|Float|Truncate (/ (Variables|BBoxData|GetBBoxXLenghtCM) 1e+02))) "by" (Utilities|String|ToString(Integer) (Math|Float|Truncate (/ (Variables|BBoxData|GetBBoxYLenghtCM) 1e+02)))))
      (CallFunction|GenerateWorldMesh (Variables|Default|GetTerrainMesh) (/ (Variables|BBoxData|GetBBoxXLenghtCM) 1e+04) (/ (Variables|BBoxData|GetBBoxYLenghtCM) 1e+04) 1e+02 0.0)
      (Rendering|Debug|DrawDebugBox "0, 0, 0" (Math|Vector|MakeVector (/ (Variables|BBoxData|GetBBoxXLenghtCM) 2.0) (/ (Variables|BBoxData|GetBBoxYLenghtCM) 2.0) 0.0) "(R=1.000000,G=0.000000,B=0.067408,A=1.000000)" "0, 0, 0" 2e+02 8e+01))))

(event EventBeginPlay
  (Variables|BBoxData|SetBBoxCenterCoords (Utilities|Struct|MakeGeographicCoordinates -73.9795 40.6975 0.0))
  ;[1 1 1] Get Coordinates
  (Variables|BBoxData|SetBBoxDistanceInKm 1e+01)
  ;[1 1 1] Get BoundingBox Coordinates String
  (bind (_bboxcoords _bboxvector) (CallFunction|CalculateBoundingBox (.longitude (Variables|BBoxData|GetBBoxCenterCoords)) (.latitude (Variables|BBoxData|GetBBoxCenterCoords)) (Variables|BBoxData|GetBBoxDistanceInKm)))
  (bind _output_get (Variables|BBoxData|SetBBoxCoords (Utilities|Struct|MakeS_BBOX_COORDS (.minlat _bboxcoords) (.minlon _bboxcoords) (.maxlat _bboxcoords) (.maxlon _bboxcoords) (.center _bboxcoords))))
  (Variables|BBoxData|SetBBoxVectors _bboxvector)
  (bind _returnvalue (CallFunction|BboxFloatstoQueryCoords (.minlat _output_get) (.minlon _output_get) (.maxlat _output_get) (.maxlon _output_get)))
  ;[1 1 1] Build Query
  (Variables|API|SetData (Utilities|String|Append "[out:json][timeout:50]; 
way[\"highway\"](" _returnvalue "); 
out geom;"))
  (bind _output_get_2 (Variables|API|SetEndpoint "https://overpass.kumi.systems/api/interpreter?data="))
  (Variables|API|SetURL_Req (Utilities|String|Append _output_get_2 (Class|VaRestLibrary|PercentEncode (Variables|API|GetData))))
  ;[1 1 1] Send Request
  (Development|PrintString (Variables|API|GetData))
  (bind _returnvalue_2 (Class|VaRestSubsystem|ConstructVaRestRequestExt (|VaRestSubsystem) "GET" "json"))
  (Class|VaRestRequestJSON|SetRequestObject _returnvalue_2)
  (Class|VaRestRequestJSON|ProcessURL _returnvalue_2 (Variables|API|GetURL_Req))
  (EventDispatchers|BindEventtoOnRequestComplete _returnvalue_2 (delegate Custom|RequestComplete)))

(event Collision|EventActorBeginOverlap
  (params (OtherActor :type Actor%20Object%20Reference)))

(event EventTick
  (params (DeltaSeconds :type Float%20%28single-precision%29)))

(fn ConstructionScript)

(fn BboxFloatstoQueryCoords
  (params (InDouble :type Float%20%28double-precision%29) (InDouble2 :type Float%20%28double-precision%29) (InDouble3 :type Float%20%28double-precision%29) (InDouble4 :type Float%20%28double-precision%29))
  (return (Utilities|String|JoinStringArray (Utilities|Array|MakeArray (Utilities|String|ToString(Float) InDouble) (Utilities|String|ToString(Float) InDouble2) (Utilities|String|ToString(Float) InDouble3) (Utilities|String|ToString(Float) InDouble4)) ",")))

(fn HandlePOIGeometry
  (params (CenterVector :type Vector) (GeometryArray :type Array%20of%20S%20Geom%20Coord%20Structures))
  (LocalVariables|SetR (Math|Random|RandomFloatinRange 0.0 1.0))
  (LocalVariables|SetG (Math|Random|RandomFloatinRange 0.0 1.0))
  (LocalVariables|SetB (Math|Random|RandomFloatinRange 0.0 1.0))
  ;[1 1 1] For Each Geometry
  (for (_array_element _array_index) GeometryArray
    (bind _enginecoordinates (Class|GeoReferencingSystem|GeographictoEngine (Class|GeoReferencingSystem|GetGeoReferencingSystem) (Utilities|Struct|MakeGeographicCoordinates (.lon _array_element) (.lat _array_element) 0.0)))
    (Development|PrintString (Utilities|String|Append "GEO " "[" (Utilities|String|ToString(Integer) _array_index) "] " (Utilities|String|ToString(Vector) "0, 0, 0")) true true "(R=1.000000,G=0.447524,B=0.868915,A=1.000000)" 1e+01)
    (Rendering|Debug|DrawDebugPoint (Math|Vector|MakeVector (- (.x _enginecoordinates) (.x CenterVector)) (- (.y _enginecoordinates) (.y CenterVector)) 1.0) 5.0 (Utilities|Struct|MakeLinearColor (LocalVariables|GetR) (LocalVariables|GetG) (LocalVariables|GetB) 1.0) 1e+03)))